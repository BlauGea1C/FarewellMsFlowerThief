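; BP_Compenion is a companion character that follows the player's third-person character.
; On BeginPlay it caches the player reference and starts FollowPlayer, which issues an AI MoveTo toward the player.
; Walk speed switches between slower when near and faster when beyond a distance threshold.
; FollowPlayer re-calls itself from MoveTo's immediate output after a one-frame-length Delay, using delta seconds stored on Tick.
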(event `self.ReceiveBeginPlay`
  (bind _asbp_third_person_character (cast `/Game/ThirdPerson/Blueprints/BP_ThirdPersonCharacter` (`GameplayStatics.GetPlayerCharacter` 0)))
  (set `self.PlayerCharacter` _asbp_third_person_character)
  (`self.FollowPlayer`))

(event `self.ReceiveTick`
  (params (DeltaSeconds :type "Float (single-precision)"))
  (set `self.Delta Seconds` DeltaSeconds))

(event `FollowPlayer`
  (bind _charactermovement (`self.CharacterMovement`))
  (if (<= (`KismetMathLibrary.Vector_Distance` (`self.K2_GetActorLocation`) (`self.K2_GetActorLocation` (`self.PlayerCharacter`))) 500.0)
    (set `CharacterMovementComponent.MaxWalkSpeed` 289.0 _charactermovement)
    (else
      (set `CharacterMovementComponent.MaxWalkSpeed` 650.0 _charactermovement)))
  (`|AIMoveTo` self (0.0 0.0 0.0) (`self.PlayerCharacter`) 100.0
    (:`then`
      (`KismetSystemLibrary.Delay` (`self.Delta Seconds`))
      (`self.FollowPlayer`))))

(fn `UserConstructionScript`)