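; Hidden platform that starts invisible and without collision, then appears or vanishes through its OnReveal and OnDisappear events.
; BeginPlay creates a dynamic M_Ocultas material instance on the Cube and zeroes its opacity.
; The OpacityAlpha timeline plays forward to fade it to a faint translucency and reverses to fade it out.
; Collision switches on or off after a short delay running alongside each fade.
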(event `self.ReceiveBeginPlay`
  (`parent.ReceiveBeginPlay`)
  (`PrimitiveComponent.SetCollisionEnabled` (`self.Cube`) "NoCollision")
  (bind _returnvalue (`PrimitiveComponent.CreateDynamicMaterialInstance` (`self.Cube`) 0 "/Game/Assets/Interactuables/Platforms/Matirials/M_Ocultas.M_Ocultas" "None"))
  (bind _output_get (set `self.Material` _returnvalue))
  (`MaterialInstanceDynamic.SetScalarParameterValue` _output_get "Opacity" 0.0))

(event `/Game/Assets/Interactuables/Platforms/BPI_Revelar.OnReveal`
  (`|ExecutionSequence`
    (:`then_0`
      (`KismetSystemLibrary.Delay` 1.0)
      (`PrimitiveComponent.SetCollisionEnabled` (`self.Cube`) "QueryAndPhysics"))
    (:`then_1`
      (bind (_direction _alpha) (`Timeline|OpacityAlpha` :!label _label)
        (:`Update`
          (`MaterialInstanceDynamic.SetScalarParameterValue` (`self.Material`) "Opacity" (`KismetMathLibrary.Lerp` 0.0 0.2 _alpha)))))))

(event `/Game/Assets/Interactuables/Platforms/BPI_Revelar.OnDisappear`
  (`|ExecutionSequence`
    (:`then_0`
      (goto _label :!via `Reverse`))
    (:`then_1`
      (`KismetSystemLibrary.Delay` 1.0)
      (`PrimitiveComponent.SetCollisionEnabled` (`self.Cube`) "NoCollision"))))

(fn `UserConstructionScript`
  (`parent.UserConstructionScript`))