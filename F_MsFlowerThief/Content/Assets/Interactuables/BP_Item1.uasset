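; BP_Item1 is a pickup that grants the player the gliding ("Planeo") ability.
; Any actor overlap fetches player 0's BP_ThirdPersonCharacter, calls ActivatePlaneo on it and destroys the item.
; End overlap hides a prompt widget and closes a gate.
; The interact-key path is inactive: BeginPlay and IA_Interact are empty, and the input-enable and widget-show logic is disconnected.
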(event `self.ReceiveBeginPlay`
  ; Al activar el imput (IA) hace la función
  ;;[0.06595 0.1244 0.15 0.5] ACTIVAR IMPUT (IA)
)

(event `EnhancedInput|/Game/Input/Actions/IA_Interact`
  (params (ActionValue :type Boolean) (ElapsedSeconds :type "Float (double-precision)") (TriggeredSeconds :type "Float (double-precision)") (InputAction :type "InputAction Object Reference" :default "/Game/Input/Actions/IA_Interact.IA_Interact"))
  ; Al activar el imput (IA) hace la función
  ;; Comprueba si estas tocando el prop
)

(event `self.ReceiveActorEndOverlap`
  (params (OtherActor :type "Actor Object Reference"))
  ; Al activar el imput (IA) hace la función
  ;; Comprueba si estas tocando el prop
  (`SceneComponent.SetVisibility` (`self.Widget`) false false)
  ;; Impide que puedas coger los items sin tocarlos
  (`/Engine/EditorBlueprintResources/StandardMacros.Gate` true :!via `Close`))

(event `self.ReceiveActorBeginOverlap`
  (params (OtherActor :type "Actor Object Reference"))
  ; Cuando recojemos el objeto hace la accion de Planeo y se destruie
  (bind _asbp_third_person_character (cast `/Game/ThirdPerson/Blueprints/BP_ThirdPersonCharacter` (`GameplayStatics.GetPlayerCharacter` 0)))
  (`/Game/ThirdPerson/Blueprints/BP_ThirdPersonCharacter.ActivatePlaneo` _asbp_third_person_character)
  (`self.K2_DestroyActor`))

(fn `UserConstructionScript`)