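; Charge point item that refills the companion's light charges (Cargas) when the main character, Vivian Clarke, overlaps it.
; BeginPlay caches the first BP_Companion, and overlap filters the other actor with an interface test against BP_VivianClarke.
; If the companion's Luz is on, it destroys every BP_RevealArea and resets charges inside that loop, so only when areas exist.
; Otherwise it resets charges directly; OnInteract only calls the parent.
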(event `/Game/Assets/Interactuables/Items/BPI_Interactuable.OnInteract`
  (`parent.OnInteract`))

(event `self.ReceiveBeginPlay`
  (`parent.ReceiveBeginPlay`)
  (bind _returnvalue (`GameplayStatics.GetActorOfClass` "/Game/Assets/Companion/BP_Companion.BP_Companion_C"))
  (set `self.BP Companion` _returnvalue))

(event `self.ReceiveActorBeginOverlap`
  (params (OtherActor :type "Actor Object Reference"))
  (if (`KismetSystemLibrary.DoesImplementInterface` OtherActor "/Game/Assets/Interactuables/BP_VivianClarke.BP_VivianClarke_C")
    (if (`/Game/Assets/Companion/BP_Companion.Luz` (`self.BP Companion`))
      (bind _outactors (`GameplayStatics.GetAllActorsOfClass` "/Game/Assets/Companion/Luminiscencia/BP_RevealArea.BP_RevealArea_C"))
      (for _array_element _outactors
        (`self.K2_DestroyActor` _array_element)
        (set `/Game/Assets/Companion/BP_Companion.Cargas` 2 (`self.BP Companion`))
        (`KismetSystemLibrary.PrintString` "BORRADAS CARGADA"))
      (else
        (bind _output_get (set `/Game/Assets/Companion/BP_Companion.Cargas` 2 (`self.BP Companion`)))
        (`KismetSystemLibrary.PrintString` (`KismetStringLibrary.Conv_IntToString` _output_get))
        (`KismetSystemLibrary.PrintString` "   CARGADA")))
    (else
      (`KismetSystemLibrary.PrintString` "NO ES PERSONATE PRINCIPAL"))))

(fn `UserConstructionScript`
  (`parent.UserConstructionScript`))