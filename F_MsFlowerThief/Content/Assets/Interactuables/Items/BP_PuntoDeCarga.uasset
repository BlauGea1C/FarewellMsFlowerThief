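; BP_PuntoDeCarga is an interactable charge point that works when an actor overlaps it, while its interact event only calls the parent.
; If BolasLuz is true, the overlap destroys actors by looping over every BP_RevealArea found in the level.
; Otherwise it sets the companion's Cargas (charges) to 2 and prints a debug message.
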(event `self.ReceiveBeginPlay`
  (`parent.ReceiveBeginPlay`))

(event `/Game/Assets/Interactuables/Items/BPI_Interactuable.OnInteract`
  (`parent.OnInteract`))

(event `self.ReceiveActorBeginOverlap`
  (params (OtherActor :type "Actor Object Reference"))
  (if (`self.BolasLuz`)
    (bind _outactors (`GameplayStatics.GetAllActorsOfClass` "/Game/Assets/Companion/Luminiscencia/BP_RevealArea.BP_RevealArea_C"))
    (for _ _outactors
      (`self.K2_DestroyActor`))
    (else
      (set `/Game/Assets/Companion/BP_Companion.Cargas` 2 (`self.BP_Companion`))
      (`KismetSystemLibrary.PrintString` " CARGADA"))))

(fn `UserConstructionScript`
  (`parent.UserConstructionScript`))