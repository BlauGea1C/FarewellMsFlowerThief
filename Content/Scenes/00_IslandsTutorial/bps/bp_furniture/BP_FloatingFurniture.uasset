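; Floating furniture prop for the islands tutorial scene that bobs, slowly tumbles and fades its material on a Reveal event.
; BeginPlay creates a dynamic material with Fade at zero and randomizes RotatingMovement on two axes.
; Two timelines alternate endlessly to drive the mesh's relative location, one playing forward and the other in reverse.
; Reveal plays a separate timeline that drives the material's Fade parameter.
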(event `self.ReceiveBeginPlay`
  (bind _returnvalue (`PrimitiveComponent.CreateDynamicMaterialInstance` (`self.Mesh`) 0 (`PrimitiveComponent.GetMaterial` (`self.Mesh`) 0) "None"))
  (bind _output_get (set `self.Material` _returnvalue))
  (`MaterialInstanceDynamic.SetScalarParameterValue` _output_get "Fade" 0.0)
  (set `RotatingMovementComponent.RotationRate` (`KismetMathLibrary.MakeRotator` (`KismetMathLibrary.RandomFloatInRange` -4.0 4.0) 0.0 (`KismetMathLibrary.RandomFloatInRange` -45.0 45.0)) (`self.RotatingMovement`))
  (bind (_direction _floatingheight) (`Timeline|FloatingHeightStart` :!label _label)
    (:`Update`
      (`SceneComponent.K2_SetRelativeLocation` (`self.Mesh`) _floatingheight false false))
    (:`Finished`
      (bind (_direction_2 _floatingheight_2) (`Timeline|FloatingHeightLoop` :!via `ReverseFromEnd`)
        (:`Update`
          (`SceneComponent.K2_SetRelativeLocation` (`self.Mesh`) _floatingheight_2 false false))
        (:`Finished`
          (goto _label :!via `PlayFromStart`))))))

(event `Reveal`
  (bind (_direction _newtrack_0) (`Timeline|Timeline`)
    (:`Update`
      (`MaterialInstanceDynamic.SetScalarParameterValue` (`self.Material`) "Fade" _newtrack_0))))

(fn `UserConstructionScript`)