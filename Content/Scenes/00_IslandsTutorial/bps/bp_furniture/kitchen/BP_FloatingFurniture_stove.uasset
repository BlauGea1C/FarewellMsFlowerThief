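; Floating kitchen stove for the islands tutorial scene, a child Blueprint whose mesh moves along an animated floating-height path.
; Each MovementAnimation call alternates through a FlipFlop between playing one timeline from the start and reversing it from the end.
; The timeline's update sets the mesh's relative location without sweeping.
; An unconnected two-timeline chain that would loop the motion back and forth continuously never runs.
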(event `self.ReceiveBeginPlay`
  (`parent.ReceiveBeginPlay`))

(event `MovementAnimation`
  (`/Engine/EditorBlueprintResources/StandardMacros.FlipFlop`
    (:`A`
      (bind (_direction _floatingheight) (`Timeline|Timeline_2` :!via `PlayFromStart` :!label _label)
        (:`Update`
          (`SceneComponent.K2_SetRelativeLocation` (`self.Mesh`) _floatingheight false false))))
    (:`B`
      (goto _label :!via `ReverseFromEnd`))))

(fn `UserConstructionScript`
  (`parent.UserConstructionScript`))