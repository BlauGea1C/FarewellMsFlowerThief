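; Floating island platform for the islands tutorial that bobs continuously and shows instructions when the player steps into its trigger box.
; Two timelines alternate, one played forward and the other in reverse, to drive the platform mesh's relative location in an endless loop.
; Box overlap creates and animates a tutorial widget, notifies a linked Island through BPI_Island, and plays the widget's hide animation on exit.
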(event `self.ReceiveBeginPlay`
  (bind (_direction _floatingheight) (`Timeline|Timeline` :!label _label)
    (:`Update`
      (`SceneComponent.K2_SetRelativeLocation` (`self.tutorial_platform__01`) _floatingheight false false))
    (:`Finished`
      (bind (_direction_2 _floatingheight_2) (`Timeline|Timeline_0` :!via `ReverseFromEnd`)
        (:`Update`
          (`SceneComponent.K2_SetRelativeLocation` (`self.tutorial_platform__01`) _floatingheight_2 false false))
        (:`Finished`
          (goto _label :!via `PlayFromStart`))))))

(event `self.Box.OnComponentBeginOverlap`
  (params (OverlappedComponent :type "PrimitiveComponent Object Reference") (OtherActor :type "Actor Object Reference") (OtherComp :type "PrimitiveComponent Object Reference") (OtherBodyIndex :type Integer) (bFromSweep :type Boolean) (SweepResult :type "HitResult Structure (by ref)"))
  (bind _island (`self.island`))
  (bind _instructiontuto (`self.InstructionTuto`))
  (if (== OtherActor (`GameplayStatics.GetPlayerCharacter` 0))
    (`KismetSystemLibrary.PrintString` "TUTO ON")
    (bind _returnvalue (`|CreateWidget` "/Game/Assets/UI_HUD/HUD/WBP_Tutorial_Instructions.WBP_Tutorial_Instructions_C" (`GameplayStatics.GetPlayerController` 0)))
    (bind _output_get (set `self.Tutorial_Instructions` _returnvalue))
    (`/Game/Assets/UI_HUD/HUD/WBP_Tutorial_Instructions.ShowTutorial` _output_get _instructiontuto)
    (`/Game/Assets/UI_HUD/HUD/WBP_Tutorial_Instructions.AnimationMostrar` _output_get _instructiontuto)
    (`UserWidget.AddToViewport` _output_get 0)
    (if (`KismetSystemLibrary.DoesImplementInterface` _island "/Game/Scenes/00_IslandsTutorial/bps/BPI_Island.BPI_Island_C")
      (`KismetSystemLibrary.PrintString` "isla on")
      (message `/Game/Scenes/00_IslandsTutorial/bps/BPI_Island.ActivateIsand` _island))))

(event `self.Box.OnComponentEndOverlap`
  (params (OverlappedComponent :type "PrimitiveComponent Object Reference") (OtherActor :type "Actor Object Reference") (OtherComp :type "PrimitiveComponent Object Reference") (OtherBodyIndex :type Integer))
  (if (== OtherActor (`GameplayStatics.GetPlayerCharacter` 0))
    (`KismetSystemLibrary.PrintString` "TUTO OFF")
    (`/Game/Assets/UI_HUD/HUD/WBP_Tutorial_Instructions.AnimationOcultar` (stale `self.Box.OnComponentBeginOverlap` _output_get) (`self.InstructionTuto`))
    (`KismetSystemLibrary.PrintString` "TUTO OFF")))

(fn `UserConstructionScript`)