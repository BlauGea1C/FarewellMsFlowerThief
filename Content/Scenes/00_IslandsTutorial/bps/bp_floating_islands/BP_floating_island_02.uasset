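; Floating island platform for the islands tutorial that stays hidden and non-collidable until activated.
; From BeginPlay, two timelines chain endlessly, one playing forward and the other in reverse, each setting the platform mesh's relative location from its FloatingHeight track.
; The custom event ActivateIsand unhides the actor and restores query and physics collision, while the floating motion runs regardless of activation.
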(event `self.ReceiveBeginPlay`
  (`self.SetActorHiddenInGame` true)
  (`PrimitiveComponent.SetCollisionEnabled` (`self.tutorial_platform__02`) "NoCollision")
  (bind (_direction _floatingheight) (`Timeline|Timeline` :!label _label)
    (:`Update`
      (`SceneComponent.K2_SetRelativeLocation` (`self.tutorial_platform__02`) _floatingheight false false))
    (:`Finished`
      (bind (_direction_2 _floatingheight_2) (`Timeline|Timeline_0` :!via `ReverseFromEnd`)
        (:`Update`
          (`SceneComponent.K2_SetRelativeLocation` (`self.tutorial_platform__02`) _floatingheight_2 false false))
        (:`Finished`
          (goto _label :!via `PlayFromStart`))))))

(event `/Game/Scenes/00_IslandsTutorial/bps/BPI_Island.ActivateIsand`
  (`self.SetActorHiddenInGame` false)
  (`PrimitiveComponent.SetCollisionEnabled` (`self.tutorial_platform__02`) "QueryAndPhysics"))

(fn `UserConstructionScript`)