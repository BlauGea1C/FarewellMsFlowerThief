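; Floating tutorial island that starts hidden and non-collidable until activated.
; Activation restores visibility and collision, fades the platform in through a timeline-driven dynamic material, and reveals floating furniture overlapping its sphere.
; Player overlap with its box shows a tutorial instructions widget and activates linked islands through BPI_Island; leaving plays the hide animation.
; The floating movement timeline is left disconnected.
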(event `self.ReceiveBeginPlay`
  (`self.SetActorHiddenInGame` true)
  (`PrimitiveComponent.SetCollisionEnabled` (`self.tutorial_platform__02`) "NoCollision")
  (`self.MovementAnimation`)
  (bind _returnvalue (`PrimitiveComponent.CreateDynamicMaterialInstance` (`self.tutorial_platform__02`) 0 "/Game/Scenes/01_Forest_Magical/02_forest_map/materials/MM_landscape_vertex_Tutorial.MM_landscape_vertex_Tutorial" "None"))
  (set `self.Material` _returnvalue))

(event `MovementAnimation`
  ; Movement
)

(event `/Game/Scenes/00_IslandsTutorial/bps/BPI_Island.ActivateIsand`
  (`self.SetActorHiddenInGame` false)
  (`PrimitiveComponent.SetCollisionEnabled` (`self.tutorial_platform__02`) "QueryAndPhysics")
  (`self.RevealIslandAndFriends`))

(event `RevealIslandAndFriends`
  (`|ExecutionSequence`
    (:`then_0`
      (`TimelineComponent.SetPlayRate` (`self.Reveal`) 1.0)
      (bind (_direction _newtrack_0) (`Timeline|Reveal`)
        (:`Update`
          (`MaterialInstanceDynamic.SetScalarParameterValue` (`self.Material`) "Fade" _newtrack_0))))
    (:`then_1`
      (for _array_element (`PrimitiveComponent.GetOverlappingActors` (`self.Sphere`) "/Game/Scenes/00_IslandsTutorial/bps/bp_furniture/BP_FloatingFurniture.BP_FloatingFurniture_C")
        (bind _asbp_floating_furniture (cast `/Game/Scenes/00_IslandsTutorial/bps/bp_furniture/BP_FloatingFurniture` _array_element))
        (`/Game/Scenes/00_IslandsTutorial/bps/bp_furniture/BP_FloatingFurniture.Reveal` _asbp_floating_furniture)))))

(event `self.Box.OnComponentBeginOverlap`
  (params (OverlappedComponent :type "PrimitiveComponent Object Reference") (OtherActor :type "Actor Object Reference") (OtherComp :type "PrimitiveComponent Object Reference") (OtherBodyIndex :type Integer) (bFromSweep :type Boolean) (SweepResult :type "HitResult Structure (by ref)"))
  (bind _instructiontuto (`self.InstructionTuto`))
  (if (== OtherActor (`GameplayStatics.GetPlayerCharacter` 0))
    (`KismetSystemLibrary.PrintString` "TUTO ON")
    (bind _returnvalue (`|CreateWidget` "/Game/Assets/UI_HUD/HUD/WBP_Tutorial_Instructions.WBP_Tutorial_Instructions_C" (`GameplayStatics.GetPlayerController` 0)))
    (bind _output_get (set `self.Tutorial_Instructions` _returnvalue))
    (`/Game/Assets/UI_HUD/HUD/WBP_Tutorial_Instructions.ShowTutorial` _output_get _instructiontuto)
    (`/Game/Assets/UI_HUD/HUD/WBP_Tutorial_Instructions.AnimationMostrar` _output_get _instructiontuto)
    (`UserWidget.AddToViewport` _output_get 0)
    (for _array_element (`self.island`)
      (if (`KismetSystemLibrary.DoesImplementInterface` _array_element "/Game/Scenes/00_IslandsTutorial/bps/BPI_Island.BPI_Island_C")
        (`KismetSystemLibrary.PrintString` "isla on")
        (message `/Game/Scenes/00_IslandsTutorial/bps/BPI_Island.ActivateIsand` _array_element)))))

(event `self.Box.OnComponentEndOverlap`
  (params (OverlappedComponent :type "PrimitiveComponent Object Reference") (OtherActor :type "Actor Object Reference") (OtherComp :type "PrimitiveComponent Object Reference") (OtherBodyIndex :type Integer))
  (if (== OtherActor (`GameplayStatics.GetPlayerCharacter` 0))
    (`KismetSystemLibrary.PrintString` "TUTO OFF")
    (`/Game/Assets/UI_HUD/HUD/WBP_Tutorial_Instructions.AnimationOcultar` (stale `self.Box.OnComponentBeginOverlap` _output_get) (`self.InstructionTuto`))
    (`KismetSystemLibrary.PrintString` "TUTO OFF")))

(fn `UserConstructionScript`)