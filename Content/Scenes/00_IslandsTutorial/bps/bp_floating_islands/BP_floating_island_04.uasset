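; Floating island platform 04 for the islands tutorial scene, which stays hidden until it is activated.
; BeginPlay hides the actor and turns off collision on its TutorialPlatform04 component.
; The ActivateIsand event unhides the actor and restores query and physics collision.
; An unconnected pair of ping-pong timelines would bob the platform through its relative location, but never runs.
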(event `self.ReceiveBeginPlay`
  (`self.SetActorHiddenInGame` true)
  (`PrimitiveComponent.SetCollisionEnabled` (`self.tutorial_platform__04`) "NoCollision"))

(event `/Game/Scenes/00_IslandsTutorial/bps/BPI_Island.ActivateIsand`
  (`self.SetActorHiddenInGame` false)
  (`PrimitiveComponent.SetCollisionEnabled` (`self.tutorial_platform__04`) "QueryAndPhysics"))

(fn `UserConstructionScript`)