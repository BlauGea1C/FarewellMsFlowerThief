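; Companion luminescence area that reveals hidden objects and protects the player inside it.
; Shortly after BeginPlay it scans its sphere's overlaps once, sending a reveal message through BPI_Revelar or, failing that, a delete message through BPI_DeleteWalls.
; Its Destroy event tells hidden platforms still overlapping the sphere to disappear again.
; Actor begin and end overlaps toggle IsProtected on the third-person character.
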(event `self.ReceiveBeginPlay`
  (`KismetSystemLibrary.Delay` 0.1)
  (for _array_element (`PrimitiveComponent.GetOverlappingActors` (`self.Sphere1`) null)
    (if (`KismetSystemLibrary.DoesImplementInterface` _array_element "/Game/Assets/Interactuables/Platforms/BPI_Revelar.BPI_Revelar_C")
      (message `/Game/Assets/Interactuables/Platforms/BPI_Revelar.OnReveal` _array_element)
      (elif (`KismetSystemLibrary.DoesImplementInterface` _array_element "/Game/Assets/Puzzles/DarkWalls/BPI_DeleteWalls.BPI_DeleteWalls_C")
        (message `/Game/Assets/Puzzles/DarkWalls/BPI_DeleteWalls.OnDelete` _array_element)))))

(event `Destroy`
  (for _array_element (`PrimitiveComponent.GetOverlappingActors` (`self.Sphere1`) "/Game/Assets/Interactuables/Platforms/BP_Platform_Ocultas.BP_Platform_Ocultas_C")
    (if (`KismetSystemLibrary.DoesImplementInterface` _array_element "/Game/Assets/Interactuables/Platforms/BPI_Revelar.BPI_Revelar_C")
      (message `/Game/Assets/Interactuables/Platforms/BPI_Revelar.OnDisappear` _array_element))))

(event `self.ReceiveActorBeginOverlap`
  (params (OtherActor :type "Actor Object Reference"))
  (bind _asbp_third_person_character (cast `/Game/ThirdPerson/Blueprints/BP_ThirdPersonCharacter` OtherActor))
  (set `/Game/ThirdPerson/Blueprints/BP_ThirdPersonCharacter.IsProtected` true _asbp_third_person_character))

(event `self.ReceiveActorEndOverlap`
  (params (OtherActor :type "Actor Object Reference"))
  (bind _asbp_third_person_character (cast `/Game/ThirdPerson/Blueprints/BP_ThirdPersonCharacter` OtherActor))
  (set `/Game/ThirdPerson/Blueprints/BP_ThirdPersonCharacter.IsProtected` false _asbp_third_person_character))

(fn `UserConstructionScript`)