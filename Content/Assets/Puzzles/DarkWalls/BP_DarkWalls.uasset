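; BP_DarkWalls is a puzzle wall that starts solid and opaque and is removed when OnDelete is called.
; BeginPlay enables collision and creates a dynamic M_DarkWalls material instance on the Cube to control its Opacity parameter.
; OnDelete disables collision after a short delay while an Opacity timeline drives that parameter.
; Both Lerp endpoints are zero, so the wall turns transparent immediately instead of fading.
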(event `self.ReceiveBeginPlay`
  (`PrimitiveComponent.SetCollisionEnabled` (`self.Cube`) "QueryAndPhysics")
  (bind _returnvalue (`PrimitiveComponent.CreateDynamicMaterialInstance` (`self.Cube`) 0 "/Game/Assets/Puzzles/DarkWalls/M_DarkWalls.M_DarkWalls" "None"))
  (bind _output_get (set `self.M_DarkWalls` _returnvalue))
  (`MaterialInstanceDynamic.SetScalarParameterValue` _output_get "Opacity" 1.0))

(event `/Game/Assets/Puzzles/DarkWalls/BPI_DeleteWalls.OnDelete`
  (`|ExecutionSequence`
    (:`then_0`
      (`KismetSystemLibrary.Delay` 1.0)
      (`PrimitiveComponent.SetCollisionEnabled` (`self.Cube`) "NoCollision"))
    (:`then_1`
      (bind (_direction _alpha) (`Timeline|Opacity`)
        (:`Update`
          (`MaterialInstanceDynamic.SetScalarParameterValue` (`self.M_DarkWalls`) "Opacity" (`KismetMathLibrary.Lerp` 0.0 0.0 _alpha)))))))

(fn `UserConstructionScript`)