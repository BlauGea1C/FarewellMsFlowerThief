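; BP_FloresMater is a puzzle wall that opens once enough switches have been activated.
; On BeginPlay it gives its Cube a dynamic dark-wall material at full opacity.
; Each Interruptor_0n event increments a counter, and reaching the required count calls OnActivate.
; A timeline then fades the material's Opacity to zero and disables the Cube's collision from its update.
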(event `self.ReceiveActorBeginOverlap`
  (params (OtherActor :type "Actor Object Reference")))

(event `self.ReceiveActorEndOverlap`
  (params (OtherActor :type "Actor Object Reference")))

(event `self.ReceiveBeginPlay`
  (bind _returnvalue (`PrimitiveComponent.CreateDynamicMaterialInstance` (`self.Cube`) 0 "/Game/Assets/Puzzles/DarkWalls/M_DarkWalls.M_DarkWalls" "None"))
  (bind _output_get (set `self.Matirial_Wall` _returnvalue))
  (`MaterialInstanceDynamic.SetScalarParameterValue` _output_get "Opacity" 1.0))

(event `Interruptor_0n`
  (`/Engine/EditorBlueprintResources/StandardMacros.IncrementInt` (`self.Interruptores_Activados`)
    (:`  `
      (if (>= (`self.Interruptores_Activados`) (`self.Interruptores_Necesarios`))
        (`self.OnActivate`)))))

(event `OnActivate`
  (bind (_direction _alpha) (`Timeline|Timeline`)
    (:`Update`
      (`MaterialInstanceDynamic.SetScalarParameterValue` (`self.Matirial_Wall`) "Opacity" (`KismetMathLibrary.Lerp` 1.0 0.0 _alpha))
      (`PrimitiveComponent.SetCollisionEnabled` (`self.Cube`) "NoCollision"))))

(fn `UserConstructionScript`)