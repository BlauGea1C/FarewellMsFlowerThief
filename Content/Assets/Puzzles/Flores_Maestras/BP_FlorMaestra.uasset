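; BP_FlorMaestra is a puzzle controller that opens a door when stones are activated in the order stored in Codigo.
; ActivarPiedra compares each stone's ID to the current code step, turning a match green, marking it activated and advancing.
; Completing the code plays a timeline that moves the Cube vertically.
; A wrong stone turns red, resets progress, then returns to blue after a short delay inside a loop over BPFlor.
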(event `/Game/Assets/Puzzles/Flores_Maestras/BPI_FlorMaestra.ActivarPiedra`
  (params (PiedraID :type Integer) (BP_Piedara :type "/Game/Assets/Puzzles/Flores_Maestras/BP_Flor Object Reference"))
  (bind _material (`/Game/Assets/Puzzles/Flores_Maestras/BP_Flor.Material` BP_Piedara))
  (if (`self.CodeOk`)
    _
    (elif (== PiedraID (`|GetArrayItem` (`self.Codigo`) (`self.Index`)))
      (`MaterialInstanceDynamic.SetVectorParameterValue` _material "Color" (struct :`G` 1.0 :`A` 1.0))
      (set `/Game/Assets/Puzzles/Flores_Maestras/BP_Flor.ActivateOk` true BP_Piedara)
      (bind _result (`/Engine/EditorBlueprintResources/StandardMacros.IncrementInt` (`self.Index`))
        (:`  `
          (bind _output_get (set `self.Index` _result))
          (if (== _output_get (`KismetArrayLibrary.Array_Length` (`self.Codigo`)))
            (`KismetSystemLibrary.PrintString` "puertaAbierta")
            (bind (_direction _doorposition) (`Timeline|Timeline`)
              (:`Update`
                (`SceneComponent.K2_SetRelativeLocation` (`self.Cube`) (`KismetMathLibrary.MakeVector` 0.0 0.0 _doorposition) false false)))
            (else
              (`KismetSystemLibrary.PrintString` "ok")))))
      (else
        (`MaterialInstanceDynamic.SetVectorParameterValue` _material "Color" (struct :`R` 1.0 :`A` 1.0))
        (set `self.Index` 0)
        (`KismetSystemLibrary.PrintString` "codigo_nocorrecto INDEX 0")
        (for _ (`self.BP_Flor`)
          (`KismetSystemLibrary.Delay` 0.2)
          (`MaterialInstanceDynamic.SetVectorParameterValue` _material "Color" (struct :`R` 0.039546 :`G` 0.127438 :`B` 0.871367 :`A` 1.0)))))))

(fn `UserConstructionScript`)