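; BP_Laser is a laser hazard that damages the player while they stand inside its Box trigger.
; BeginPlay caches the player as BP_ThirdPersonCharacter, and only that actor triggers the overlap logic.
; Entering the box calls Daño at once and starts a looping timer that repeats it, cutting health through the player's HealthManager and printing a debug message.
; Leaving the box clears the timer to stop the damage.
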(event `self.ReceiveBeginPlay`
  (bind _asbp_third_person_character (cast `/Game/ThirdPerson/Blueprints/BP_ThirdPersonCharacter` (`GameplayStatics.GetPlayerCharacter` 0)))
  (set `self.Player` _asbp_third_person_character))

(event `Daño`
  (`/Game/ThirdPerson/Blueprints/BP_ThirdPersonCharacter.HealthManager` (`self.Player`) -0.75)
  (`KismetSystemLibrary.PrintString` "DAÑO"))

(event `self.Box.OnComponentBeginOverlap`
  (params (OverlappedComponent :type "PrimitiveComponent Object Reference") (OtherActor :type "Actor Object Reference") (OtherComp :type "PrimitiveComponent Object Reference") (OtherBodyIndex :type Integer) (bFromSweep :type Boolean) (SweepResult :type "HitResult Structure (by ref)"))
  (if (== OtherActor (`self.Player`))
    (set `self.IsLaser` true)
    (if (`self.IsLaser`)
      (`self.Daño`)
      (bind _returnvalue (`KismetSystemLibrary.K2_SetTimerDelegate` (delegate `Daño`) 5.0 true)))))

(event `self.Box.OnComponentEndOverlap`
  (params (OverlappedComponent :type "PrimitiveComponent Object Reference") (OtherActor :type "Actor Object Reference") (OtherComp :type "PrimitiveComponent Object Reference") (OtherBodyIndex :type Integer))
  (if (== OtherActor (`self.Player`))
    (set `self.IsLaser` false)
    (`KismetSystemLibrary.K2_ClearAndInvalidateTimerHandle` (stale `self.Box.OnComponentBeginOverlap` _returnvalue))))

(fn `UserConstructionScript`)