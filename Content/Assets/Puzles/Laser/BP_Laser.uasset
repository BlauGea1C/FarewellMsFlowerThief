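; BP_Laser is a laser hazard that switches on and off on a looping timer and damages the player.
; Each toggle activates or deactivates the Posion effect and the Box collision together.
; When the player overlaps the Box, damage applies immediately and repeats on a timer until the overlap ends.
; Each hit calls the player's HealthManager, shows an animated damage widget and advances the lives UI through the laser's own hit counter.
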(event `ON/OFF`
  (set `self.LaserActivo` (not (`self.LaserActivo`)))
  (if (`self.LaserActivo`)
    (`ActorComponent.Activate` (`self.Posion`) false)
    (`PrimitiveComponent.SetCollisionEnabled` (`self.Box`) "QueryOnly")
    (else
      (`ActorComponent.Deactivate` (`self.Posion`))
      (`PrimitiveComponent.SetCollisionEnabled` (`self.Box`) "NoCollision"))))

(event `Daño`
  (`/Game/ThirdPerson/Blueprints/BP_ThirdPersonCharacter.HealthManager` (`self.Player`) 1.0)
  (bind _returnvalue (`|CreateWidget` "/Game/Assets/UI_HUD/HUD/WBP_Damage.WBP_Damage_C"))
  (bind _output_get (set `self.MenuDamege` _returnvalue))
  (`UserWidget.AddToViewport` _output_get 0)
  (`/Game/Assets/UI_HUD/HUD/WBP_Damage.AnimationDamege` _output_get)
  (bind _result (`/Engine/EditorBlueprintResources/StandardMacros.IncrementInt` (`self.Index`))
    (:`  `
      (bind _output_get_2 (set `self.Index` _result))
      (`/Game/Assets/UI_HUD/HUD/WBP_HUD.SwitchWidgetVidas` (`/Game/ThirdPerson/Blueprints/BP_ThirdPersonCharacter.UI` (`self.Player`)) _output_get_2))))

(event `self.ReceiveBeginPlay`
  (bind _asbp_third_person_character (cast `/Game/ThirdPerson/Blueprints/BP_ThirdPersonCharacter` (`GameplayStatics.GetPlayerCharacter` 0)))
  (set `self.Player` _asbp_third_person_character)
  (`KismetSystemLibrary.K2_SetTimerDelegate` (delegate `ON/OFF`) (`self.TimerON/OFF`) true))

(event `self.Box.OnComponentBeginOverlap`
  (params (OverlappedComponent :type "PrimitiveComponent Object Reference") (OtherActor :type "Actor Object Reference") (OtherComp :type "PrimitiveComponent Object Reference") (OtherBodyIndex :type Integer) (bFromSweep :type Boolean) (SweepResult :type "HitResult Structure (by ref)"))
  (if (== OtherActor (`self.Player`))
    (set `self.IsLaser` true)
    (if (`self.IsLaser`)
      (`self.Daño`)
      (bind _returnvalue (`KismetSystemLibrary.K2_SetTimerDelegate` (delegate `Daño`) 2.0 true)))))

(event `self.Box.OnComponentEndOverlap`
  (params (OverlappedComponent :type "PrimitiveComponent Object Reference") (OtherActor :type "Actor Object Reference") (OtherComp :type "PrimitiveComponent Object Reference") (OtherBodyIndex :type Integer))
  (if (== OtherActor (`self.Player`))
    (set `self.IsLaser` false)
    (`KismetSystemLibrary.K2_ClearAndInvalidateTimerHandle` (stale `self.Box.OnComponentBeginOverlap` _returnvalue))))

(fn `UserConstructionScript`)