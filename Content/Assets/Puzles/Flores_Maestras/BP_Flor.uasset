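; BP_Flor is an interactable puzzle piece that the player triggers by overlapping it, reporting to a master flower.
; A DoOnce sends its PiedraID and itself to BPFlorMaestra until ResetInteraction re-arms it.
; ActivateEmissive plays a timeline driving the crystal's dynamic material EmissiveIntensity on Correct, and reverses it on Incorrect or Restore.
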(event `self.ReceiveBeginPlay`
  (bind _returnvalue (`PrimitiveComponent.CreateDynamicMaterialInstance` (`self.puzzle_code_crystals`) 0 "/Game/Assets/Forest/minerals_crystals/M_crystal_pink_Puzzle.M_crystal_pink_Puzzle" "None"))
  (set `self.Material` _returnvalue))

(event `self.ReceiveActorBeginOverlap`
  (params (OtherActor :type "Actor Object Reference"))
  (if (== OtherActor (`GameplayStatics.GetPlayerCharacter` 0))
    (`/Engine/EditorBlueprintResources/StandardMacros.DoOnce` false :!label _label
      (:`Completed`
        (message `/Game/Assets/Puzles/Flores_Maestras/BPI_Inteructores.ActivarPiedra` (`self.BP_FlorMaestra`) (`self.PiedraID`) self)))))

(event `ResetInteraction`
  (goto _label :!via `Reset`))

(event `ActivateEmissive`
  (params (State :type "/Game/Assets/Puzles/Flores_Maestras/Enum_CrystalStates Enum" :default "NewEnumerator0"))
  (switch `/Game/Assets/Puzles/Flores_Maestras/Enum_CrystalStates` State
    (:`NewEnumerator0`
      (bind (_direction _alpha) (`Timeline|EmissiveAnimation` :!label _label_2)
        (:`Update`
          (`MaterialInstanceDynamic.SetScalarParameterValue` (`self.Material`) "EmissiveIntensity" (`KismetMathLibrary.Lerp` 0.0 0.75 _alpha)))))
    (:`NewEnumerator1`
      (goto _label_2 :!via `Reverse`))
    (:`NewEnumerator2`
      (goto _label_2 :!via `Reverse`))))

(fn `UserConstructionScript`)