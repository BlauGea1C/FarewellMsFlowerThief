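; BP_FlorMaestra is the master flower of a sequence puzzle that opens a door.
; ActivarPiedra records each interactor and checks its ID against the next Codigo entry, lighting it when correct.
; Completing the code plays, after a delay, a timeline that moves the Cube door vertically and destroys the Niagara component.
; A wrong ID briefly flashes, then resets every recorded interactor and, after an index-scaled delay, restarts the sequence.
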(event `self.ReceiveTick`
  (params (DeltaSeconds :type "Float (single-precision)")))

(event `/Game/Assets/Puzles/Flores_Maestras/BPI_Inteructores.ActivarPiedra`
  (params (InterucotrID :type Integer) (BP_Inteructor :type "/Game/Assets/Puzles/Flores_Maestras/BP_Flor Object Reference"))
  (if (not (`self.CodeOk`))
    (`KismetArrayLibrary.Array_Add` (`self.BP_Flor`))
    (if (== InterucotrID (`|GetArrayItem` (`self.Codigo`) (`self.Index`)))
      (`/Game/Assets/Puzles/Flores_Maestras/BP_Flor.ActivateEmissive` BP_Inteructor "NewEnumerator0")
      (bind _result (`/Engine/EditorBlueprintResources/StandardMacros.IncrementInt` (`self.Index`))
        (:`  `
          (if (== _result (`KismetArrayLibrary.Array_Length` (`self.Codigo`)))
            (`KismetSystemLibrary.Delay` 1.0)
            (`KismetSystemLibrary.PrintString` "puertaAbierta")
            (bind (_direction _doorposition) (`Timeline|Timeline`)
              (:`Update`
                (`SceneComponent.K2_SetRelativeLocation` (`self.Cube`) (`KismetMathLibrary.MakeVector` 0.0 0.0 _doorposition) false false)
                (`ActorComponent.K2_DestroyComponent` (`self.Niagara`))))
            (else
              (`KismetSystemLibrary.PrintString` "ok")))))
      (else
        (`/Game/Assets/Puzles/Flores_Maestras/BP_Flor.ActivateEmissive` BP_Inteructor "NewEnumerator0")
        (`KismetSystemLibrary.Delay` 0.2)
        (`/Game/Assets/Puzles/Flores_Maestras/BP_Flor.ActivateEmissive` BP_Inteructor "NewEnumerator2")
        (`KismetSystemLibrary.PrintString` "codigo_nocorrecto INDEX 0")
        (for _array_element (`self.BP_Flor`)
          (`/Game/Assets/Puzles/Flores_Maestras/BP_Flor.ActivateEmissive` _array_element "NewEnumerator2")
          (`/Game/Assets/Puzles/Flores_Maestras/BP_Flor.ResetInteraction` _array_element))
        (`KismetSystemLibrary.Delay` (* (`self.Index`) 0.5))
        (`KismetArrayLibrary.Array_Clear` (`self.BP_Flor`))
        (set `self.Index` 0)))))

(fn `UserConstructionScript`)