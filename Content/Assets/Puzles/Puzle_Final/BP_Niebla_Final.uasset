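; Final-puzzle barrier actor that moves its Cube out like a door once enough switches are activated.
; On BeginPlay it counts all BP_Interector_Final actors in the level as the required total.
; ActivateSwitch records IDs and calls OpenDoor when their count matches, otherwise it calls DeactivateSwitch with a fixed ID of 0.
; OpenDoor plays a Timeline that drives the Cube's relative Z location.
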(event `self.ReceiveBeginPlay`
  (bind _outactors (`GameplayStatics.GetAllActorsOfClass` "/Game/Assets/Puzles/Puzle_Final/BP_Interector_Final.BP_Interector_Final_C"))
  (bind _output_get (set `self.BP_Inteructor_Finel` _outactors))
  (set `self.NumInterucotores` (`KismetArrayLibrary.Array_Length` _output_get)))

(event `ActivateSwitch`
  (params (ID_Inteructor :type Integer))
  (`KismetArrayLibrary.Array_Add` (`self.IDsActivados`) ID_Inteructor)
  (`KismetSystemLibrary.PrintString` "holaaaa")
  (if (== (`KismetArrayLibrary.Array_Length` (`self.IDsActivados`)) (`self.NumInterucotores`))
    (`self.OpenDoor`)
    (else
      (`self.DeactivateSwitch` 0))))

(event `DeactivateSwitch`
  (params (ID :type Integer))
  (`KismetArrayLibrary.Array_RemoveItem` (`self.IDsActivados`) ID))

(event `OpenDoor`
  (`KismetSystemLibrary.PrintString` "puertaAbierta")
  (bind (_direction _doorposition) (`Timeline|Timeline`)
    (:`Update`
      (`SceneComponent.K2_SetRelativeLocation` (`self.Cube`) (`KismetMathLibrary.MakeVector` 0.0 0.0 _doorposition) false false))))

(fn `UserConstructionScript`)