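; Puzzle door that opens once every BP_Interector_One_Line switch in the level has been activated, with no repeats.
; BeginPlay gathers and counts those switches.
; ActivateSwitch records each new ID and updates that switch's emissive state; a repeated ID clears progress and switches the emissive state on all of them.
; When the recorded count matches the total, OpenDoor plays a Timeline that moves the Cube's relative Z.
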(event `self.ReceiveBeginPlay`
  (bind _outactors (`GameplayStatics.GetAllActorsOfClass` "/Game/Assets/Puzles/Puerta_Interruptores/BP_Interector_One_Line.BP_Interector_One_Line_C"))
  (bind _output_get (set `self.BP_Inteructor_One_Line` _outactors))
  (set `self.NumInterucotores` (`KismetArrayLibrary.Array_Length` _output_get)))

(event `ActivateSwitch`
  (params (ID_Inteructor :type Integer) (BP_Interucotr :type "/Game/Assets/Puzles/Puerta_Interruptores/BP_Interector_One_Line Object Reference"))
  (if (`KismetArrayLibrary.Array_Contains` (`self.IDsActivados`) ID_Inteructor)
    (`self.ResetPuzzle`)
    (`KismetSystemLibrary.PrintString` "PUZLE REINICUADO")
    (else
      (`KismetArrayLibrary.Array_Add` (`self.IDsActivados`) ID_Inteructor)
      (`KismetSystemLibrary.PrintString` "Inteructro ON")
      (`/Game/Assets/Puzles/Puerta_Interruptores/BP_Interector_One_Line.Emissive` BP_Interucotr "NewEnumerator0")
      (if (== (`KismetArrayLibrary.Array_Length` (`self.IDsActivados`)) (`self.NumInterucotores`))
        (`self.OpenDoor`)))))

(event `ResetPuzzle`
  (`KismetArrayLibrary.Array_Clear` (`self.IDsActivados`))
  (`/Game/Assets/Puzles/Puerta_Interruptores/BP_Interector_One_Line.Emissive` (`self.BP_Inteructor_One_Line`) "NewEnumerator1"))

(event `OpenDoor`
  (`KismetSystemLibrary.PrintString` "puertaAbierta")
  (bind (_direction _doorposition) (`Timeline|Timeline`)
    (:`Update`
      (`SceneComponent.K2_SetRelativeLocation` (`self.Cube`) (`KismetMathLibrary.MakeVector` 0.0 0.0 _doorposition) false false))))

(fn `UserConstructionScript`)