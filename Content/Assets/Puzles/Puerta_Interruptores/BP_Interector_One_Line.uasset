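; Crystal switch actor for the one-line door puzzle, identified by an ID.
; On overlap it passes its ID and itself to BPPuertaOneLine through ActivateSwitch and prints a debug string.
; BeginPlay creates a dynamic material on the crystal mesh.
; The Emissive event plays a timeline that ramps that material's glow up on Activado and reverses it on Restart.
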(event `self.ReceiveBeginPlay`
  (bind _returnvalue (`PrimitiveComponent.CreateDynamicMaterialInstance` (`self.crystal_chunk_01`) 0 "/Game/Assets/Forest/crystal_chunks/M_crystal_blue_puzle.M_crystal_blue_puzle" "None"))
  (set `self.Material` _returnvalue))

(event `self.ReceiveActorBeginOverlap`
  (params (OtherActor :type "Actor Object Reference"))
  (`/Game/Assets/Puzles/Puerta_Interruptores/BP_Puerta_One_Line.ActivateSwitch` (`self.BP_Puerta_One_Line`) (`self.ID`) self)
  (`KismetSystemLibrary.PrintString` "interucotrON"))

(event `Emissive`
  (params (State :type "/Game/Assets/Puzles/Puerta_Interruptores/OneLine Enum" :default "NewEnumerator0"))
  (switch `/Game/Assets/Puzles/Puerta_Interruptores/OneLine` State
    (:`NewEnumerator0`
      (bind (_direction _alpha) (`Timeline|Timeline` :!label _label)
        (:`Update`
          (`MaterialInstanceDynamic.SetScalarParameterValue` (`self.Material`) "EmissiveIntensity" (`KismetMathLibrary.Lerp` 0.0 1.0 _alpha)))))
    (:`NewEnumerator1`
      (goto _label :!via `Reverse`))))

(fn `UserConstructionScript`)