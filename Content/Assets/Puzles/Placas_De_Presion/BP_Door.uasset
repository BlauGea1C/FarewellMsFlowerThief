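; BP_Door is a puzzle door that moves vertically when enough pressure switches are active at once.
; SwichActivate and SwitchDesactivate raise or lower the active switch count and compare it to PressureSwitchesNeeded.
; The DoorActivete timeline plays when the threshold is met and reverses otherwise, driving the Door component's relative Z location.
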(event `SwichActivate`
  ;[0.05145 0.15 0.006089 0.5] Si el numero de pulsadores es igual al numero de pulsadores que se necesita para abrir la puerta se abre la puerta
  (`/Engine/EditorBlueprintResources/StandardMacros.IncrementInt` (`self.PressureSwitchesActive`)
    (:`  `
      (if (>= (`self.PressureSwitchesActive`) (`self.PressureSwitchesNeeded`))
        ; Animacion
        (bind (_direction _doorposition) (`Timeline|DoorActivete` :!label _label)
          (:`Update`
            (`SceneComponent.K2_SetRelativeLocation` (`self.Door`) (`KismetMathLibrary.MakeVector` 0.0 0.0 _doorposition) false false)))
        (else
          (goto _label :!via `Reverse`))))))

(event `SwitchDesactivate`
  ;[0.15 0.07657 0.002121 0.5] Si el ya no se presiona el numero de pulsadores necesario la puera se ciera
  (`/Engine/EditorBlueprintResources/StandardMacros.DecrementInt` (`self.PressureSwitchesActive`)
    (:`  `
      (if (>= (`self.PressureSwitchesActive`) (`self.PressureSwitchesNeeded`))
        (goto _label)
        (else
          (goto _label :!via `Reverse`))))))

(fn `UserConstructionScript`)