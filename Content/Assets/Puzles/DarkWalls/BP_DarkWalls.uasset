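; BP_DarkWalls is a puzzle wall that fades away and opens once enough switches have been activated.
; BeginPlay gives the VfxWall mesh a dynamic M_vfx_wall material at full opacity.
; Each Interruptor_0n event increments a counter, and reaching InterruptoresNecesarios calls OnActivate.
; OnActivate plays a timeline that lerps opacity to zero, disabling collision and setting Open from its update.
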(event `self.ReceiveBeginPlay`
  (bind _returnvalue (`PrimitiveComponent.CreateDynamicMaterialInstance` (`self.vfx_wall`) 0 "/Game/Assets/Puzles/DarkWalls/M_vfx_wall.M_vfx_wall" "None"))
  (bind _output_get (set `self.Matirial_Wall` _returnvalue))
  (`MaterialInstanceDynamic.SetScalarParameterValue` _output_get "Opacity" 1.0))

(event `self.ReceiveActorBeginOverlap`
  (params (OtherActor :type "Actor Object Reference")))

(event `self.ReceiveActorEndOverlap`
  (params (OtherActor :type "Actor Object Reference")))

(event `Interruptor_0n`
  (`/Engine/EditorBlueprintResources/StandardMacros.IncrementInt` (`self.Interruptores_Activados`)
    (:`  `
      (if (>= (`self.Interruptores_Activados`) (`self.Interruptores_Necesarios`))
        ; al revés
        (`self.OnActivate`)))))

(event `OnActivate`
  (bind (_direction _alpha) (`Timeline|Timeline`)
    (:`Update`
      (`MaterialInstanceDynamic.SetScalarParameterValue` (`self.Matirial_Wall`) "Opacity" (`KismetMathLibrary.Lerp` 1.0 0.0 _alpha))
      (`PrimitiveComponent.SetCollisionEnabled` (`self.vfx_wall`) "NoCollision")
      (set `self.Open` true))))

(fn `UserConstructionScript`)