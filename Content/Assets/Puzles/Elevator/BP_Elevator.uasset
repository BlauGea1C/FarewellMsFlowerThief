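; BP_Elevator is a puzzle wind elevator that floats the third-person character upward while it is inside a capsule.
; If switched on, capsule entry inverts the character's gravity, sets upward velocity and adds a downward force; exit restores a fixed gravity scale.
; SwitchON/OFF toggles the state, which is checked only on entry.
; Logic to swap dandelion Niagara effects exists but is unconnected.
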(event `self.Capsule.OnComponentBeginOverlap`
  (params (OverlappedComponent :type "PrimitiveComponent Object Reference") (OtherActor :type "Actor Object Reference") (OtherComp :type "PrimitiveComponent Object Reference") (OtherBodyIndex :type Integer) (bFromSweep :type Boolean) (SweepResult :type "HitResult Structure (by ref)"))
  (`KismetSystemLibrary.PrintString` "Elevador")
  (if (`self.IsElevatorON`)
    (bind _asbp_third_person_character (cast `/Game/ThirdPerson/Blueprints/BP_ThirdPersonCharacter` OtherActor))
    (bind _charactermovement (`Character.CharacterMovement` _asbp_third_person_character))
    (set `CharacterMovementComponent.GravityScale` -1.0 _charactermovement)
    (set `MovementComponent.Velocity` (0.0 0.0 100.0) _charactermovement)
    (`CharacterMovementComponent.AddForce` _charactermovement (0.0 0.0 -100.0))))

(event `self.Capsule.OnComponentEndOverlap`
  (params (OverlappedComponent :type "PrimitiveComponent Object Reference") (OtherActor :type "Actor Object Reference") (OtherComp :type "PrimitiveComponent Object Reference") (OtherBodyIndex :type Integer))
  (bind _asbp_third_person_character (cast `/Game/ThirdPerson/Blueprints/BP_ThirdPersonCharacter` OtherActor))
  (set `CharacterMovementComponent.GravityScale` 1.75 (`Character.CharacterMovement` _asbp_third_person_character)))

(event `SwitchON/OFF`
  (if (`self.IsElevatorON`)
    (set `self.IsElevatorON` false)
    (else
      (set `self.IsElevatorON` true))))

(fn `UserConstructionScript`)