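; BP_ToxicZone1 is a hazard zone that periodically damages the player while they stay inside it.
; Overlap begin and end toggle a damage-zone flag for the cached third-person player character.
; A looping one-second Delay calls the player's HealthManager with a negative amount and prints a debug message, skipping damage while the player is protected.
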(event `self.ReceiveBeginPlay`
  (bind _asbp_third_person_character (cast `/Game/ThirdPerson/Blueprints/BP_ThirdPersonCharacter` (`GameplayStatics.GetPlayerCharacter` 0)))
  (set `self.Player` _asbp_third_person_character))

(event `self.ReceiveActorBeginOverlap`
  (params (OtherActor :type "Actor Object Reference"))
  (if (== OtherActor (`self.Player`))
    (set `self.IsDamageZone` true)
    (`KismetSystemLibrary.Delay` 1.0 :!label _label)
    (if (`self.IsDamageZone`)
      (if (`/Game/ThirdPerson/Blueprints/BP_ThirdPersonCharacter.IsProtected` (`self.Player`))
        (goto _label)
        (else
          (`/Game/ThirdPerson/Blueprints/BP_ThirdPersonCharacter.HealthManager` (`self.Player`) -0.5)
          (`KismetSystemLibrary.PrintString` "DAÑO")
          (goto _label))))))

(event `self.ReceiveActorEndOverlap`
  (params (OtherActor :type "Actor Object Reference"))
  (if (== OtherActor (`self.Player`))
    (set `self.IsDamageZone` false)))

(fn `UserConstructionScript`)