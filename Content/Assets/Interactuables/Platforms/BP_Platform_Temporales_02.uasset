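; Temporary platform made of four petal meshes that falls away shortly after anything overlaps its trigger box.
; After a short delay, four timelines lerp each petal straight down in relative space.
; Each timeline starts the next from its Update pin, so the petals drop almost together rather than sequentially.
; The last timeline's Update also disables collision on all petals; nothing resets the platform.
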(event `self.ReceiveBeginPlay`)

(event `self.Box.OnComponentBeginOverlap`
  (params (OverlappedComponent :type "PrimitiveComponent Object Reference") (OtherActor :type "Actor Object Reference") (OtherComp :type "PrimitiveComponent Object Reference") (OtherBodyIndex :type Integer) (bFromSweep :type Boolean) (SweepResult :type "HitResult Structure (by ref)"))
  (`KismetSystemLibrary.Delay` 1.5)
  (bind (_direction _alpha) (`Timeline|Position_Petalo_01`)
    (:`Update`
      (`SceneComponent.K2_SetRelativeLocation` (`self.Plataformas_temporales_petalo_01`) (`KismetMathLibrary.VLerp` (28.148925 32.025368 0.0) (28.148925 32.025368 -500.0) _alpha) false false)
      (bind (_direction_2 _alpha_2) (`Timeline|Timeline`)
        (:`Update`
          (`SceneComponent.K2_SetRelativeLocation` (`self.Plataformas_temporales_petalo_02`) (`KismetMathLibrary.VLerp` (28.148925 -31.040359 0.0) (28.148925 -31.040359 -500.0) _alpha_2) false false)
          (bind (_direction_3 _alpha_3) (`Timeline|Timeline_0`)
            (:`Update`
              (`SceneComponent.K2_SetRelativeLocation` (`self.Plataformas_temporales_petalo_03`) (`KismetMathLibrary.VLerp` (-31.514927 -31.040364 0.0) (-31.514927 -31.040364 -500.0) _alpha_3) false false)
              (bind (_direction_4 _alpha_4) (`Timeline|Timeline_1`)
                (:`Update`
                  (`SceneComponent.K2_SetRelativeLocation` (`self.Plataformas_temporales_petalo_04`) (`KismetMathLibrary.VLerp` (-31.514927 32.025363 0.0) (-31.514927 32.025363 -500.0) _alpha_4) false false)
                  (`PrimitiveComponent.SetCollisionEnabled` (`self.Plataformas_temporales_petalo_01`) "NoCollision")
                  (`PrimitiveComponent.SetCollisionEnabled` (`self.Plataformas_temporales_petalo_02`) "NoCollision")
                  (`PrimitiveComponent.SetCollisionEnabled` (`self.Plataformas_temporales_petalo_03`) "NoCollision")
                  (`PrimitiveComponent.SetCollisionEnabled` (`self.Plataformas_temporales_petalo_04`) "NoCollision"))))))))))

(fn `UserConstructionScript`)