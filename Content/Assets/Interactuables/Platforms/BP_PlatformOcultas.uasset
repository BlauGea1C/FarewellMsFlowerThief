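; BP_PlatformOcultas is a hidden platform that starts invisible and non-collidable, then appears or vanishes through OnReveal and OnDisappear.
; A timeline fades the dynamic material's opacity to a faint translucency and reverses it to hide.
; Box collision switches on or off after a one-second delay in each direction.
; The construction script gives InterpToMovement control points at its origin and relative MoveToPos for platform movement.
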(event `self.ReceiveBeginPlay`
  (`PrimitiveComponent.SetCollisionEnabled` (`self.Box`) "NoCollision")
  (bind _returnvalue (`PrimitiveComponent.CreateDynamicMaterialInstance` (`self.Box`) 0 "/Game/Assets/Interactuables/Platforms/Matirials/M_Ocultas.M_Ocultas" "None"))
  (bind _output_get (set `self.Matirial` _returnvalue))
  (`MaterialInstanceDynamic.SetScalarParameterValue` _output_get "Opacity" 0.0))

(event `/Game/Assets/Interactuables/Platforms/BPI_Revelar.OnReveal`
  (`|ExecutionSequence`
    (:`then_0`
      (`KismetSystemLibrary.Delay` 1.0)
      (`PrimitiveComponent.SetCollisionEnabled` (`self.Box`) "QueryAndPhysics"))
    (:`then_1`
      (bind (_direction _alpha) (`Timeline|Timeline` :!label _label)
        (:`Update`
          (`MaterialInstanceDynamic.SetScalarParameterValue` (`self.Matirial`) "Opacity" (`KismetMathLibrary.Lerp` 0.0 0.2 _alpha)))))))

(event `/Game/Assets/Interactuables/Platforms/BPI_Revelar.OnDisappear`
  (`|ExecutionSequence`
    (:`then_0`
      (goto _label :!via `Reverse`))
    (:`then_1`
      (`KismetSystemLibrary.Delay` 1.0)
      (`PrimitiveComponent.SetCollisionEnabled` (`self.Box`) "NoCollision"))))

(fn `UserConstructionScript`
  (`InterpToMovementComponent.AddControlPointPosition` (`self.InterpToMovement`) (0.0 0.0 0.0) true)
  (`InterpToMovementComponent.AddControlPointPosition` (`self.InterpToMovement`) (`self.MoveToPos`) true))