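; Base interactable item actor that shows a prompt widget while the player character, Vivian, overlaps it.
; On interaction, collectible items open a paused WBP_Collectibles screen, update Vivian's book UI and send cycling dialogue lines through the character when its speaking check is false.
; PickUpItem destroys the actor and returns its name.
; The interact input, DialogueSpeak and both speaking-check functions are stubs, and DestoyActor only delays.
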(event `self.ReceiveBeginPlay`
  ; Al activar el imput (IA) hace la función
  ;;[0.06595 0.1244 0.15 0.5] ACTIVAR IMPUT (IA)
  (`self.EnableInput` (`GameplayStatics.GetPlayerController` 0))
  (bind _asbp_third_person_character (cast `/Game/ThirdPerson/Blueprints/BP_ThirdPersonCharacter` (`GameplayStatics.GetPlayerCharacter` 0)))
  (set `self.Vivian` _asbp_third_person_character))

(event `EnhancedInput|/Game/Inputs/Actions/IA_Interact`
  (params (ActionValue :type Boolean) (ElapsedSeconds :type "Float (double-precision)") (TriggeredSeconds :type "Float (double-precision)") (InputAction :type "InputAction Object Reference" :default "/Game/Inputs/Actions/IA_Interact.IA_Interact"))
  ; Al activar el imput (IA) hace la función
  ;; Comprueba si estas tocando el prop
)

(event `self.ReceiveActorBeginOverlap`
  (params (OtherActor :type "Actor Object Reference"))
  ; Al activar el imput (IA) hace la función
  (`/Game/Utilities/BPML_Utilities.IsVivian?` OtherActor
    (:`true`
      (`SceneComponent.SetVisibility` (`self.Widget`) true false)
      ;; Impide que puedas coger los items sin tocarlos
      (`/Engine/EditorBlueprintResources/StandardMacros.Gate` true :!via `Open` :!label _label))))

(event `self.ReceiveActorEndOverlap`
  (params (OtherActor :type "Actor Object Reference"))
  ; Al activar el imput (IA) hace la función
  (`/Game/Utilities/BPML_Utilities.IsVivian?` OtherActor
    (:`true`
      (`SceneComponent.SetVisibility` (`self.Widget`) false false)
      (goto _label :!via `Close`))))

(event `/Game/Assets/Interactuables/Items/BPI_Interactuable.OnInteract`
  (bind _returnvalue (`GameplayStatics.GetPlayerCharacter` 0))
  (bind _dialogue (`self.Dialogue`))
  (bind _ui (`/Game/ThirdPerson/Blueprints/BP_ThirdPersonCharacter.UI` (`self.Vivian`)))
  ; Al activar el imput (IA) hace la función
  (`KismetSystemLibrary.PrintString` (`KismetSystemLibrary.GetDisplayName` self))
  (if (`self.IsCollectible`)
    (`KismetSystemLibrary.PrintString` "SI C")
    (bind _returnvalue_2 (`|CreateWidget` "/Game/Assets/UI_HUD/HUD/WBP_Collectibles.WBP_Collectibles_C"))
    (bind _output_get (set `self.Collectibles` _returnvalue_2))
    (`UserWidget.AddToViewport` _output_get 0)
    (`/Game/Assets/UI_HUD/HUD/WBP_Collectibles.SetNameCollectible` _output_get (`self.Text`))
    (set `/Game/Assets/UI_HUD/HUD/WBP_Collectibles.IsOpen` true _output_get)
    (`GameplayStatics.SetGamePaused` true)
    (`WidgetBlueprintLibrary.SetInputMode_GameAndUIEx` (`GameplayStatics.GetPlayerController` 0) _output_get)
    (`Widget.SetKeyboardFocus` _output_get)
    (bind _output_get_2 (set `self.IndexBook` 1))
    (`/Game/Assets/UI_HUD/HUD/WBP_HUD.SwitchWidgetBook` _ui _output_get_2)
    (`/Game/Assets/UI_HUD/HUD/WBP_HUD.AnimationBook` _ui 0)
    (bind _bspeakingcollectible (message `/Game/Assets/Interactuables/Items/BPI_Interactuable.CheckingSpeakingCollectible` _returnvalue))
    (`KismetSystemLibrary.PrintString` "CheckingSpeaking")
    (if (not _bspeakingcollectible)
      (`KismetSystemLibrary.PrintString` "CHECKING TRUE")
      (message `/Game/Assets/Interactuables/Items/BPI_Interactuable.SpeakingCollectibles` _returnvalue (`|GetArrayItem` _dialogue (`self.CurrentIndex`)) (`self.TextDelay`))
      (bind _result (`/Engine/EditorBlueprintResources/StandardMacros.IncrementInt` (`self.CurrentIndex`))
        (:`  `
          (if (>= _result (`KismetArrayLibrary.Array_Length` _dialogue))
            (set `self.CurrentIndex` 0)))))
    (else
      (`KismetSystemLibrary.PrintString` "NO C"))))

(event `/Game/Assets/Interactuables/Items/BPI_Interactuable.SpeakingCollectibles`
  (params (Dialogue :type String) (TextDelay :type "Float (double-precision)"))
  ; Al activar el imput (IA) hace la función
  (message `/Game/Assets/Interactuables/Items/BPI_Interactuable.SpeakingCollectibles` (`self.Collectibles`) Dialogue TextDelay))

(event `DestoyActor`
  ; Al activar el imput (IA) hace la función
  (`KismetSystemLibrary.Delay` 0.1))

(event `DialogueSpeak`
  ; Al activar el imput (IA) hace la función
)

(fn `CheckingSpeaking`
  (returns (bSpeaking :type Boolean))
  (return false))

(fn `CheckingSpeakingCollectible`
  (returns (bSpeakingCollectible :type Boolean))
  (return false))

(fn `PickUpItem`
  (returns (Item :type String))
  (`KismetSystemLibrary.PrintString` "Itenm Pick Up")
  (`self.K2_DestroyActor`)
  (return (`self.itemName`)))

(fn `UserConstructionScript`)