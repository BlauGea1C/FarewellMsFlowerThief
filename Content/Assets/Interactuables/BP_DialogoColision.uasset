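; Trigger-volume actor that has the player character speak a dialogue line on entering its box.
; The overlap runs through a DoOnce with no reset, so it fires once, even if the line is skipped because a message is already showing.
; It passes the current Dialogue entry and TextDelay to the player's SpeakingMessage, then advances the index with wraparound.
; Debug prints remain in the flow.
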(event `self.Box.OnComponentBeginOverlap`
  (params (OverlappedComponent :type "PrimitiveComponent Object Reference") (OtherActor :type "Actor Object Reference") (OtherComp :type "PrimitiveComponent Object Reference") (OtherBodyIndex :type Integer) (bFromSweep :type Boolean) (SweepResult :type "HitResult Structure (by ref)"))
  (bind _returnvalue (`GameplayStatics.GetPlayerCharacter` 0))
  (bind _dialogue (`self.Dialogue`))
  (if (== OtherActor (`GameplayStatics.GetPlayerCharacter` 0))
    (`/Engine/EditorBlueprintResources/StandardMacros.DoOnce` false
      (:`Completed`
        (bind _bspeaking (message `/Game/Assets/Interactuables/Items/BPI_Interactuable.CheckingSpeaking` _returnvalue))
        (`KismetSystemLibrary.PrintString` "CheckingSpeaking")
        (if (not _bspeaking)
          (`KismetSystemLibrary.PrintString` "CHECKING TRUE")
          (message `/Game/Assets/Interactuables/Items/BPI_Interactuable.Speaking` _returnvalue (`|GetArrayItem` _dialogue (`self.CurrentIndex`)) (`self.TextDelay`))
          (bind _result (`/Engine/EditorBlueprintResources/StandardMacros.IncrementInt` (`self.CurrentIndex`))
            (:`  `
              (if (>= _result (`KismetArrayLibrary.Array_Length` _dialogue))
                (set `self.CurrentIndex` 0)))))))))

(fn `UserConstructionScript`)