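; BP_moving_platform1 is a moving platform that travels from its placed location toward a point displaced by MoveOffset.
; On BeginPlay it stores both endpoints and plays the TL_Move timeline, whose Alpha lerps the actor location on each update without sweep.
; Unconnected InterpToMovement control-point nodes remain in the construction script and never run.
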(event `self.ReceiveBeginPlay`
  (bind _output_get (set `self.PointA` (`self.K2_GetActorLocation`)))
  (set `self.PointB` (+ _output_get (`self.MoveOffset`)))
  (bind (_direction _alpha) (`Timeline|TL_Move`)
    (:`Update`
      (`self.K2_SetActorLocation` (`KismetMathLibrary.VLerp` (`self.PointA`) (`self.PointB`) _alpha)))))

(fn `UserConstructionScript`)