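; Temporary platform made of four petals that dissolves when Vivian overlaps its box, then reforms.
; BeginPlay gives all petals one shared dynamic dissolve material, so a single parameter drives their fade.
; The overlap plays the Dissolve timeline while delays switch petal collision off partway through.
; RestorePetalos later reverses the timeline and re-enables collision after another delay.
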(event `self.ReceiveBeginPlay`
  (bind _returnvalue (`KismetMaterialLibrary.CreateDynamicMaterialInstance` "/Game/VFX/Systems/Dissolve/M_DissolvePetals.M_DissolvePetals"))
  (bind _output_get (set `self.Plataformas_temporales_petalo_01_Mat` _returnvalue))
  (`PrimitiveComponent.SetMaterial` (`self.Plataformas_temporales_petalo_01`) 0 _output_get)
  (`PrimitiveComponent.SetMaterial` (`self.Plataformas_temporales_petalo_02`) 0 _output_get)
  (`PrimitiveComponent.SetMaterial` (`self.Plataformas_temporales_petalo_03`) 0 _output_get)
  (`PrimitiveComponent.SetMaterial` (`self.Plataformas_temporales_petalo_04`) 0 _output_get)
  (`MaterialInstanceDynamic.SetScalarParameterValue` _output_get "Dissolve" (`self.ValueDissolve`)))

(event `self.Box.OnComponentBeginOverlap`
  (params (OverlappedComponent :type "PrimitiveComponent Object Reference") (OtherActor :type "Actor Object Reference") (OtherComp :type "PrimitiveComponent Object Reference") (OtherBodyIndex :type Integer) (bFromSweep :type Boolean) (SweepResult :type "HitResult Structure (by ref)"))
  (`/Game/Utilities/BPML_Utilities.IsVivian?` OtherActor
    (:`true`
      (`|ExecutionSequence`
        (:`then_0`
          (`KismetSystemLibrary.Delay` 1.5)
          (`PrimitiveComponent.SetCollisionEnabled` (`self.Plataformas_temporales_petalo_01`) "NoCollision")
          (`PrimitiveComponent.SetCollisionEnabled` (`self.Plataformas_temporales_petalo_02`) "NoCollision")
          (`PrimitiveComponent.SetCollisionEnabled` (`self.Plataformas_temporales_petalo_03`) "NoCollision")
          (`PrimitiveComponent.SetCollisionEnabled` (`self.Plataformas_temporales_petalo_04`) "NoCollision")
          (`KismetSystemLibrary.Delay` 2.0)
          (`self.RestorePetalos`))
        (:`then_1`
          (bind (_direction _dissolvetrack) (`Timeline|Dissolve` :!label _label)
            (:`Update`
              (`MaterialInstanceDynamic.SetScalarParameterValue` (`self.Plataformas_temporales_petalo_01_Mat`) "Dissolve" (`KismetMathLibrary.Lerp` -1.0 1.0 _dissolvetrack)))))))))

(event `RestorePetalos`
  (`|ExecutionSequence`
    (:`then_0`
      (goto _label :!via `Reverse`))
    (:`then_1`
      (`KismetSystemLibrary.Delay` 1.5)
      (`PrimitiveComponent.SetCollisionEnabled` (`self.Plataformas_temporales_petalo_01`) "QueryAndPhysics")
      (`PrimitiveComponent.SetCollisionEnabled` (`self.Plataformas_temporales_petalo_02`) "QueryAndPhysics")
      (`PrimitiveComponent.SetCollisionEnabled` (`self.Plataformas_temporales_petalo_03`) "QueryAndPhysics")
      (`PrimitiveComponent.SetCollisionEnabled` (`self.Plataformas_temporales_petalo_04`) "QueryAndPhysics"))))

(fn `UserConstructionScript`)