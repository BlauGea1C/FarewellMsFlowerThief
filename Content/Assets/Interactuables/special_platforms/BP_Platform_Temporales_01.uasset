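; BP_Platform_Temporales_01 is a temporary platform that glows, animates its opacity and destroys itself after being touched.
; BeginPlay creates a dynamic material on the Cube from M_PlatformsTemporales, with brightness off.
; Any Box overlap raises brightness through the misspelled "Birght" parameter and plays a timeline driving Opacity.
; A one-second delay, started alongside that timeline, then destroys the actor.
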(event `self.ReceiveBeginPlay`
  (bind _returnvalue (`PrimitiveComponent.CreateDynamicMaterialInstance` (`self.Cube`) 0 "/Game/Assets/Interactuables/special_platforms/textures/M_PlatformsTemporales.M_PlatformsTemporales" "None"))
  (bind _output_get (set `self.DynamicMatirial` _returnvalue))
  (`MaterialInstanceDynamic.SetScalarParameterValue` _output_get "Birght" 0.0))

(event `self.Box.OnComponentBeginOverlap`
  (params (OverlappedComponent :type "PrimitiveComponent Object Reference") (OtherActor :type "Actor Object Reference") (OtherComp :type "PrimitiveComponent Object Reference") (OtherBodyIndex :type Integer) (bFromSweep :type Boolean) (SweepResult :type "HitResult Structure (by ref)"))
  (`MaterialInstanceDynamic.SetScalarParameterValue` (`self.DynamicMatirial`) "Birght" 10.0)
  (`|ExecutionSequence`
    (:`then_0`
      (bind (_direction _opacity) (`Timeline|Timeline_Opacity`)
        (:`Update`
          (`MaterialInstanceDynamic.SetScalarParameterValue` (`self.DynamicMatirial`) "Opacity" _opacity))))
    (:`then_1`
      (`KismetSystemLibrary.Delay` 1.0)
      (`self.K2_DestroyActor`))))

(fn `UserConstructionScript`)