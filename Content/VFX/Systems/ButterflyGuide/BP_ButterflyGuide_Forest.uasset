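; Butterfly guide actor that appears when the third-person character touches it and flies from one point to another.
; A dynamic material on the origami butterfly starts invisible, then a timeline fades it to half opacity while a Niagara effect activates.
; Delays chained from timeline updates start the move between PointA and PointB, then a fade-out and the actor's destruction.
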(event `self.ReceiveBeginPlay`
  (bind _returnvalue (`PrimitiveComponent.CreateDynamicMaterialInstance` (`self.origami_butterfly`) 0 "/Game/VFX/Systems/ButterflyGuide/M_ButterflyGuide.M_ButterflyGuide" "None"))
  (bind _output_get (set `self.Material` _returnvalue))
  (`MaterialInstanceDynamic.SetScalarParameterValue` _output_get "Opacity" 0.0))

(event `self.ButterflyCollision.OnComponentBeginOverlap`
  (params (OverlappedComponent :type "PrimitiveComponent Object Reference") (OtherActor :type "Actor Object Reference") (OtherComp :type "PrimitiveComponent Object Reference") (OtherBodyIndex :type Integer) (bFromSweep :type Boolean) (SweepResult :type "HitResult Structure (by ref)"))
  (cast `/Game/ThirdPerson/Blueprints/BP_ThirdPersonCharacter` OtherActor)
  (bind (_direction _alpha) (`Timeline|Timeline`)
    (:`Update`
      (`MaterialInstanceDynamic.SetScalarParameterValue` (`self.Material`) "Opacity" (`KismetMathLibrary.Lerp` 0.0 0.5 _alpha))
      (`ActorComponent.Activate` (`self.NS_ButterflyGuide`) false)
      (`KismetSystemLibrary.Delay` 2.0)
      (bind (_direction_2 _location_track) (`Timeline|Jump Timeline First Island` :!via `PlayFromStart`)
        (:`Update`
          (`self.K2_SetActorLocation` (`KismetMathLibrary.VLerp` (`self.K2_GetActorLocation` (`self.Point_A`)) (`self.K2_GetActorLocation` (`self.Point_B`)) _location_track))
          (`KismetSystemLibrary.Delay` 5.0)
          (bind (_direction_3 _alpha_2) (`Timeline|Timeline_0` :!via `PlayFromStart`)
            (:`Update`
              (`MaterialInstanceDynamic.SetScalarParameterValue` (`self.Material`) "Opacity" (`KismetMathLibrary.Lerp` 0.5 0.0 _alpha_2))
              (`KismetSystemLibrary.Delay` 2.0)
              (`self.K2_DestroyActor`))))))))

(fn `UserConstructionScript`)